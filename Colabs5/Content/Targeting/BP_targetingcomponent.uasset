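; Targeting component that gives its owning Character a toggleable lock-on to nearby actors implementing the targeting interface.
; A sphere trace gathers candidates, then camera line traces and a view-direction dot product pick the target.
; While locked, character rotation follows the controller, which Tick turns toward the target.
; Left/right switching filters by hit normal against camera right, though the right switch only clears the target.
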(event `self.ReceiveBeginPlay`
  (bind _ascharacter (cast `Character` (`self.GetOwner`)))
  (set `self.Character Ref` _ascharacter)
  (set `self.Camera ref` (`Actor.GetComponentByClass` (`self.Character Ref`) "/Script/Engine.CameraComponent")))

(event `Lockontoactorleft`
  (bind _closesttarget (`self.Find closest targetOntheleft` (`self.Find actors to lock on to`)))
  (`/Engine/EditorBlueprintResources/StandardMacros.IsValid` (`self.Locked on actor`)
    (:`Is Valid`
      (`/Engine/EditorBlueprintResources/StandardMacros.IsValid` _closesttarget
        (:`Is Valid`
          (set `self.Locked on actor` _closesttarget))
        (:`Is Not Valid`
          (`self.Stop lock on`))))))

(event `Lockontoactorright`
  (`/Engine/EditorBlueprintResources/StandardMacros.IsValid` (`self.Locked on actor`)
    (:`Is Valid`
      (`/Engine/EditorBlueprintResources/StandardMacros.IsValid` (`self.Find closest targetOntheright` (`self.Find actors to lock on to`))
        (:`Is Valid`
          (set `self.Locked on actor` null))
        (:`Is Not Valid`
          (`self.Stop lock on`))))))

(event `Lock on to target`
  (bind _closesttarget (`self.Find closest target` (`self.Find actors to lock on to`)))
  (`/Engine/EditorBlueprintResources/StandardMacros.IsValid` _closesttarget
    (:`Is Valid`
      (set `self.Locked on actor` _closesttarget)
      (`self.Orient camera`)
      (set `self.LockedOn?` true))))

(event `Orient camera`
  (bind _charactermovement (`Character.CharacterMovement` (`self.Character Ref`)))
  (set `CharacterMovementComponent.bOrientRotationToMovement` false _charactermovement)
  (set `CharacterMovementComponent.bUseControllerDesiredRotation` true _charactermovement))

(event `Stop lock on`
  (set `self.Locked on actor` null)
  (set `self.LockedOn?` false)
  (`self.Orient movement`))

(event `Orient movement`
  (bind _charactermovement (`Character.CharacterMovement` (`self.Character Ref`)))
  (set `CharacterMovementComponent.bOrientRotationToMovement` true _charactermovement)
  (set `CharacterMovementComponent.bUseControllerDesiredRotation` false _charactermovement))

(event `self.ReceiveTick`
  (params (DeltaSeconds :type "Float (single-precision)"))
  (if (`self.LockedOn?`)
    (`self.Face Locked On Actor`)))

(event `Toggle lock on`
  (if (`self.LockedOn?`)
    (`self.Stop lock on`)
    (else
      (`self.Lock on to target`))))

(fn `Check how close target is to player`
  (params (Target :type "Actor Object Reference"))
  (returns (ReturnValue :type "Float (double-precision)"))
  (return (`KismetMathLibrary.Dot_VectorVector` (`SceneComponent.GetForwardVector` (`self.Camera ref`)) (`KismetMathLibrary.Conv_RotatorToVector` (`KismetMathLibrary.FindLookAtRotation` (`Actor.K2_GetActorLocation` (`self.Character Ref`)) (`Actor.K2_GetActorLocation` Target))))))

(fn `Face Locked On Actor`
  (bind _character_ref (`self.Character Ref`))
  (bind _returnvalue (`Pawn.GetController` _character_ref))
  (bind _returnvalue_2 (`Controller.GetControlRotation` _returnvalue))
  (`Controller.SetControlRotation` _returnvalue (`KismetMathLibrary.MakeRotator` (.roll _returnvalue_2) (.pitch (`KismetMathLibrary.RInterpTo_Constant` _returnvalue_2 (`KismetMathLibrary.FindLookAtRotation` (`Actor.K2_GetActorLocation` _character_ref) (`Actor.K2_GetActorLocation` (`self.Locked on actor`))) (`GameplayStatics.GetWorldDeltaSeconds`) (`self.Interp Speed`))) (.yaw (`KismetMathLibrary.RInterpTo_Constant` _returnvalue_2 (`KismetMathLibrary.FindLookAtRotation` (`Actor.K2_GetActorLocation` _character_ref) (`Actor.K2_GetActorLocation` (`self.Locked on actor`))) (`GameplayStatics.GetWorldDeltaSeconds`) (`self.Interp Speed`))))))

(fn `Find actors to lock on to`
  (returns (`Targeting actors` :type "Array of Actor Object Reference"))
  (locals (Potentialtargetingactors :type "Array of Actor Object Reference"))
  (bind _returnvalue (`Actor.K2_GetActorLocation` (`self.Character Ref`)))
  (bind (_outhits _returnvalue_2) (`KismetSystemLibrary.SphereTraceMultiForObjects` _returnvalue _returnvalue (`self.Radius`) (`|MakeArray` "ObjectTypeQuery7" :!type "EObjectTypeQuery Enum") false (`|MakeArray` (`self.GetOwner`))))
  (for _array_element _outhits
    (bind (_bblockinghit _binitialoverlap _time _distance _location _impactpoint _normal _impactnormal _physmat _hitactor) (`GameplayStatics.BreakHitResult` _array_element))
    (if (and _returnvalue_2 (`KismetSystemLibrary.DoesImplementInterface` _hitactor "/Game/Targeting/BP_targertinginterface.BP_targertinginterface_C"))
      (`KismetArrayLibrary.Array_Add` (`local.Potentialtargetingactors`) _hitactor)))
  (return (`local.Potentialtargetingactors`)))

(fn `Find closest target`
  (params (Actors :type "Array of Actor Object Reference"))
  (returns (closesttarget :type "Actor Object Reference"))
  (locals (`Compare target` :type "Float (double-precision)") (`Closest target` :type "Actor Object Reference"))
  (for _array_element Actors
    (bind (_outhit _returnvalue) (`KismetSystemLibrary.LineTraceSingle` :`Start` (`SceneComponent.K2_GetComponentLocation` (`self.Camera ref`)) :`End` (`Actor.K2_GetActorLocation` _array_element) :`TraceChannel` "TraceTypeQuery1" :`DrawDebugType` "ForDuration"))
    (if _returnvalue
      (bind _returnvalue_2 (`self.Check how close target is to player` _array_element))
      (`/Engine/EditorBlueprintResources/StandardMacros.CompareFloat` _returnvalue_2 (`local.Compare target`)
        (:`>`
          (set `local.Compare target` _returnvalue_2)
          (set `local.Closest target` _array_element)))))
  (return (`local.Closest target`)))

(fn `Find closest targetOntheleft`
  (params (Actors :type "Array of Actor Object Reference"))
  (returns (closesttarget :type "Actor Object Reference"))
  (locals (`Compare target` :type "Float (double-precision)") (`Closest target` :type "Actor Object Reference"))
  (bind _compare_target (`local.Compare target`))
  (for _array_element Actors
    (bind (_outhit _returnvalue) (`KismetSystemLibrary.LineTraceSingle` :`Start` (`SceneComponent.K2_GetComponentLocation` (`self.Camera ref`)) :`End` (`Actor.K2_GetActorLocation` _array_element) :`TraceChannel` "TraceTypeQuery1" :`DrawDebugType` "ForDuration"))
    (if (and _returnvalue (> (`KismetMathLibrary.Dot_VectorVector` (`SceneComponent.GetRightVector` (`self.Camera ref`)) (`.Normal` (`GameplayStatics.BreakHitResult` _outhit))) 0.0) (!= (`self.Locked on actor`) _array_element))
      (`/Engine/EditorBlueprintResources/StandardMacros.CompareFloat` (`self.Check how close target is to player` _array_element) _compare_target
        (:`>`
          (set `local.Compare target` _compare_target)
          (set `local.Closest target` _array_element)))))
  (return (`local.Closest target`)))

(fn `Find closest targetOntheright`
  (params (Actors :type "Array of Actor Object Reference"))
  (returns (closesttarget :type "Actor Object Reference"))
  (locals (`Compare target` :type "Float (double-precision)") (`Closest target` :type "Actor Object Reference"))
  (bind _compare_target (`local.Compare target`))
  (for _array_element Actors
    (bind (_outhit _returnvalue) (`KismetSystemLibrary.LineTraceSingle` :`Start` (`SceneComponent.K2_GetComponentLocation` (`self.Camera ref`)) :`End` (`Actor.K2_GetActorLocation` _array_element) :`TraceChannel` "TraceTypeQuery1" :`DrawDebugType` "ForDuration"))
    (if (and _returnvalue (< (`KismetMathLibrary.Dot_VectorVector` (`SceneComponent.GetRightVector` (`self.Camera ref`)) (`.Normal` (`GameplayStatics.BreakHitResult` _outhit))) 0.0) (!= (`self.Locked on actor`) _array_element))
      (`/Engine/EditorBlueprintResources/StandardMacros.CompareFloat` (`self.Check how close target is to player` _array_element) _compare_target
        (:`>`
          (set `local.Compare target` _compare_target)
          (set `local.Closest target` _array_element)))))
  (return (`local.Closest target`)))